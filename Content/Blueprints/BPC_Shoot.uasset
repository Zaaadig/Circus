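; Actor component for a charge-and-release ball-throwing attraction, limited to three balls.
; Holding IA_Shoot shows the cursor, spawns a BP_Ball at the BP_AttractionTrigger camera and starts a looping timer that builds strength up to a maximum, mirrored in a progress bar.
; Releasing stops the timer, enables the ball's physics and applies an impulse along the deprojected mouse direction, scaled by strength.
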(event `self.ReceiveBeginPlay`
  ;[1 1 1] Initialisation
  (bind _returnvalue (`|CreateWidget` "/Game/UI/Widget/WB_ProgressBarStrenght.WB_ProgressBarStrenght_C"))
  (bind _output_get (set `self.ProgressBarRef` _returnvalue))
  (`UserWidget.AddToViewport` _output_get 0)
  (`Widget.SetVisibility` (`self.ProgressBarRef`) "Collapsed")
  (bind _returnvalue_2 (`GameplayStatics.GetActorOfClass` "/Game/ThirdPerson/Blueprints/BP_ThirdPersonCharacter.BP_ThirdPersonCharacter_C"))
  (set `self.CharaRef` _returnvalue_2)
  (bind _returnvalue_3 (`GameplayStatics.GetActorOfClass` "/Game/Blueprints/BP_AttractionTrigger.BP_AttractionTrigger_C"))
  (set `self.Ref_Trigger` _returnvalue_3))

(event `EnhancedInput|/Game/ThirdPerson/Input/Actions/IA_Shoot`
  (params (ActionValue :type Boolean) (ElapsedSeconds :type "Float (double-precision)") (TriggeredSeconds :type "Float (double-precision)") (InputAction :type "InputAction Object Reference" :default "/Game/ThirdPerson/Input/Actions/IA_Shoot.IA_Shoot"))
  (bind _returnvalue (`GameplayStatics.GetPlayerController` 0))
  (bind _canshoot_ (`self.CanShoot?`))
  ;[1 1 1] Spawn de la balle
  (:`Triggered`
    (if (and _canshoot_ (<= (`self.BallLeft`) 2))
      (set `PlayerController.bShowMouseCursor` true _returnvalue)
      (`/Engine/EditorBlueprintResources/StandardMacros.DoOnce` false :!label _label
        (:`Completed`
          (bind _returnvalue_2 (`|SpawnActorFromClass` "/Game/Blueprints/BP_Ball.BP_Ball_C" (`KismetMathLibrary.MakeTransform` (`SceneComponent.K2_GetComponentLocation` (`/Game/Blueprints/BP_AttractionTrigger.Camera` (`self.Ref_Trigger`)))) "Undefined" "MultiplyWithRoot" null null))
          (set `self.RefBall` _returnvalue_2)
          (`self.AddStrenght`)))))
  (:`Completed`
    (if _canshoot_
      (`self.StopTimer`)
      (set `PlayerController.bShowMouseCursor` false _returnvalue)
      (set `self.CanAddStrenght?` true)
      (set `self.Strenght` 0.0)
      (goto _label :!via `Reset`))))

(event `ThrowBall`
  (bind _returnvalue (`GameplayStatics.GetPlayerController` 0))
  (bind (_locationx _locationy) (`PlayerController.GetMousePosition` _returnvalue))
  (bind _sphere (`/Game/Blueprints/BP_Ball.Sphere` (`self.RefBall`)))
  ;[1 1 1] Impulsion de la balle
  (`/Engine/EditorBlueprintResources/StandardMacros.IsValid` null
    (:`Is Not Valid`
      (`PrimitiveComponent.SetSimulatePhysics` _sphere true)
      (`PrimitiveComponent.SetEnableGravity` _sphere true)
      (`PrimitiveComponent.SetCollisionEnabled` _sphere "QueryAndPhysics")
      (`PrimitiveComponent.AddImpulse` _sphere (* (`.WorldDirection` (`GameplayStatics.DeprojectScreenToWorld` _returnvalue (`KismetMathLibrary.MakeVector2D` _locationx _locationy))) (`self.Strenght`)) "None" false)
      (bind _output_get (set `self.BallLeft` (+ (`self.BallLeft`) 1)))
      (if (>= _output_get 3)
        (set `self.CanShoot?` false)))))

(event `StopTimer`
  ;[1 1 1] Gestion de la force du tir
  (`KismetSystemLibrary.K2_ClearAndInvalidateTimerHandle` (stale `AddStrenght` _returnvalue))
  (`self.ThrowBall`)
  (`self.ResetProgressBar` (`self.ProgressBarRef`)))

(event `AddStrenght`
  ;[1 1 1] Gestion de la force du tir
  (bind _returnvalue (`KismetSystemLibrary.K2_SetTimerDelegate` (delegate `CodeStrenght`) 0.1 true)))

(event `/Game/Blueprints/BPI/BPI_Score.BarVisible`
  (`Widget.SetVisibility` (`self.ProgressBarRef`) "Visible"))

(event `CodeStrenght`
  ;[1 1 1] Gestion de la force du tir
  (if (`self.CanAddStrenght?`)
    (bind _output_get (set `self.Strenght` (+ (`self.Strenght`) 1000.0)))
    (`self.AdjustProgressBar` (`self.Strenght`) (`self.MaxStrenght`) (`self.ProgressBarRef`))
    (if (> _output_get (`self.MaxStrenght`))
      (set `self.CanAddStrenght?` false))))

(event `/Game/Blueprints/BPI/BPI_Score.BarInvisible`
  (`Widget.SetVisibility` (`self.ProgressBarRef`) "Collapsed"))

(fn `AdjustProgressBar`
  (params (Strenght :type "Float (double-precision)") (MaxStrenght :type "Float (double-precision)") (NewParam :type "/Game/UI/Widget/WB_ProgressBarStrenght Object Reference"))
  (`ProgressBar.SetPercent` (`/Game/UI/Widget/WB_ProgressBarStrenght.ProgressBar_0` NewParam) (/ Strenght MaxStrenght)))

(fn `ResetProgressBar`
  (params (ProgressBar :type "/Game/UI/Widget/WB_ProgressBarStrenght Object Reference"))
  (`ProgressBar.SetPercent` (`/Game/UI/Widget/WB_ProgressBarStrenght.ProgressBar_0` ProgressBar) 0.0))