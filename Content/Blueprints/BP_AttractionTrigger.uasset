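; BP_AttractionTrigger is a trigger box that starts and ends a knock-down (chamboule-tout) shooting attraction for the player.
; On overlap, it blends the view to the attraction camera, enables BPC_Shoot, shows its bar and spawns BP_Target at the BP_RefTransform position.
; On exit, it restores the player view, disables shooting, destroys the target, hides the bar and resets every BP_Score actor's score and color.
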(event `self.ReceiveBeginPlay`
  (bind _returnvalue (`GameplayStatics.GetActorOfClass` "/Game/Blueprints/BP_RefTransform.BP_RefTransform_C"))
  (set `self.RefBasePos` _returnvalue)
  (bind _outactors (`GameplayStatics.GetAllActorsOfClass` "/Game/Blueprints/BP_Score.BP_Score_C"))
  (set `self.RefScore` _outactors)
  (bind _returnvalue_2 (`GameplayStatics.GetActorOfClass` "/Game/ThirdPerson/Blueprints/BP_ThirdPersonCharacter.BP_ThirdPersonCharacter_C"))
  (set `self.RefChara` _returnvalue_2))

(event `self.Box.OnComponentBeginOverlap`
  (params (OverlappedComponent :type "PrimitiveComponent Object Reference") (OtherActor :type "Actor Object Reference") (OtherComp :type "PrimitiveComponent Object Reference") (OtherBodyIndex :type Integer) (bFromSweep :type Boolean) (SweepResult :type "HitResult Structure (by ref)"))
  ;[1 1 1] Création du chamboule tout
  (if (`self.ActorHasTag` OtherActor "Player")
    (`PlayerController.SetViewTargetWithBlend` (`GameplayStatics.GetPlayerController` 0) (`ActorComponent.GetOwner` (`self.Camera`)) 1.0 "VTBlend_Linear" 0.0 false)
    (bind _returnvalue (`GameplayStatics.GetActorOfClass` "/Game/ThirdPerson/Blueprints/BP_ThirdPersonCharacter.BP_ThirdPersonCharacter_C"))
    (bind _asbpc_shoot (cast `/Game/Blueprints/BPC_Shoot` (`/Game/ThirdPerson/Blueprints/BP_ThirdPersonCharacter.BPC_Shoot` _returnvalue)))
    (set `/Game/Blueprints/BPC_Shoot.CanShoot?` true _asbpc_shoot)
    (set `/Game/Blueprints/BPC_Shoot.BallLeft` 0 _asbpc_shoot)
    (bind _returnvalue_2 (`|SpawnActorFromClass` "/Game/Blueprints/BP_Target.BP_Target_C" (`SceneComponent.K2_GetComponentToWorld` (`Actor.RootComponent` (`self.RefBasePos`))) "Undefined" "MultiplyWithRoot" null null))
    (set `self.RefTarget` _returnvalue_2)
    (message `/Game/Blueprints/BPI/BPI_Score.BarVisible` (`/Game/ThirdPerson/Blueprints/BP_ThirdPersonCharacter.BPC_Shoot` (`self.RefChara`)))))

(event `self.Box.OnComponentEndOverlap`
  (params (OverlappedComponent :type "PrimitiveComponent Object Reference") (OtherActor :type "Actor Object Reference") (OtherComp :type "PrimitiveComponent Object Reference") (OtherBodyIndex :type Integer))
  (bind _returnvalue (`GameplayStatics.GetPlayerController` 0))
  ;[1 1 1] Création du chamboule tout
  (if (`self.ActorHasTag` OtherActor "Player")
    (`PlayerController.SetViewTargetWithBlend` _returnvalue (`Controller.K2_GetPawn` _returnvalue) 1.0 "VTBlend_Linear" 0.0 false)
    (bind _returnvalue_2 (`GameplayStatics.GetActorOfClass` "/Game/ThirdPerson/Blueprints/BP_ThirdPersonCharacter.BP_ThirdPersonCharacter_C"))
    (bind _asbpc_shoot (cast `/Game/Blueprints/BPC_Shoot` (`/Game/ThirdPerson/Blueprints/BP_ThirdPersonCharacter.BPC_Shoot` _returnvalue_2)))
    (set `/Game/Blueprints/BPC_Shoot.CanShoot?` false _asbpc_shoot)
    (set `/Game/Blueprints/BPC_Shoot.BallLeft` 0 _asbpc_shoot)
    (`self.K2_DestroyActor` (`self.RefTarget`))
    (for _array_element (`self.RefScore`)
      (message `/Game/Blueprints/BPI/BPI_Score.CastScore` _array_element 0.0)
      (message `/Game/Blueprints/BPI/BPI_Score.ResetColor` _array_element)
      (message `/Game/Blueprints/BPI/BPI_Score.BarInvisible` (`/Game/ThirdPerson/Blueprints/BP_ThirdPersonCharacter.BPC_Shoot` (`self.RefChara`))))))

(fn `UserConstructionScript`)