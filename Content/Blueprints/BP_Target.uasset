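; BP_Target is a target actor that scores when components tagged "Cans" leave its Box volume.
; On BeginPlay it caches every BP_Score actor in RefScore.
; Each qualifying end overlap increments Score, gated by a cast to BP_Score, then passes the new value to every cached actor through CastScoreMessage.
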(event `self.ReceiveBeginPlay`
  (bind _outactors (`GameplayStatics.GetAllActorsOfClass` "/Game/Blueprints/BP_Score.BP_Score_C"))
  (set `self.RefScore` _outactors))

(event `self.Box.OnComponentEndOverlap`
  (params (OverlappedComponent :type "PrimitiveComponent Object Reference") (OtherActor :type "Actor Object Reference") (OtherComp :type "PrimitiveComponent Object Reference") (OtherBodyIndex :type Integer))
  ;[1 1 1] Cast du score
  (if (`ActorComponent.ComponentHasTag` OtherComp "Cans")
    (castclass `/Game/Blueprints/BP_Score` "/Game/Blueprints/BP_Score.BP_Score_C")
    (bind _output_get (set `self.Score` (+ (`self.Score`) 1.0)))
    (for _array_element (`self.RefScore`)
      (message `/Game/Blueprints/BPI/BPI_Score.CastScore` _array_element _output_get))))

(fn `UserConstructionScript`)