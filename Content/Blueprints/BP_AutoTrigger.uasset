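; Trigger volume that puts the player in control of a random car when an actor tagged Player enters its box.
; The overlap possesses one of the first five BP_Car actors cached at BeginPlay, adds the IMC_Auto input context and shows a WB_Timer widget.
; ResetPosess returns control to the cached character and removes that context; moving the character above the car is left unwired.
; The construction script adjusts the box's X/Y scale and line thickness.
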(event `self.ReceiveBeginPlay`
  (bind _returnvalue (`GameplayStatics.GetActorOfClass` "/Game/ThirdPerson/Blueprints/BP_ThirdPersonCharacter.BP_ThirdPersonCharacter_C"))
  (set `self.PlayerRef` _returnvalue)
  (bind _outactors (`GameplayStatics.GetAllActorsOfClass` "/Game/Blueprints/BP_Car.BP_Car_C"))
  (set `self.CarsRef` _outactors))

(event `self.Box.OnComponentBeginOverlap`
  (params (OverlappedComponent :type "PrimitiveComponent Object Reference") (OtherActor :type "Actor Object Reference") (OtherComp :type "PrimitiveComponent Object Reference") (OtherBodyIndex :type Integer) (bFromSweep :type Boolean) (SweepResult :type "HitResult Structure (by ref)"))
  (bind _returnvalue (`GameplayStatics.GetPlayerController` 0))
  (if (`self.ActorHasTag` OtherActor "Player")
    (bind _output_get (set `self.CarChosen` (`KismetMathLibrary.RandomIntegerInRange` 0 4)))
    (bind _output_get_2 (set `self.CurentCar` (`|GetArrayItem` (`self.CarsRef`) _output_get)))
    (`Controller.Possess` _returnvalue (`self.CurentCar`))
    (`EnhancedInputSubsystemInterface.AddMappingContext` (pcsubsystem `EnhancedInputLocalPlayerSubsystem` _returnvalue) "/Game/ThirdPerson/Input/IMC_Auto.IMC_Auto" 0 (struct))
    (bind _returnvalue_2 (`|CreateWidget` "/Game/UI/Widget/WB_Timer.WB_Timer_C"))
    (`UserWidget.AddToViewport` _returnvalue_2 0)))

(event `/Game/Blueprints/BPI/BPI_Auto.ResetPosess`
  (bind _returnvalue (`GameplayStatics.GetPlayerController` 0))
  (`Controller.Possess` _returnvalue (`self.PlayerRef`))
  (`EnhancedInputSubsystemInterface.RemoveMappingContext` (pcsubsystem `EnhancedInputLocalPlayerSubsystem` _returnvalue) "/Game/ThirdPerson/Input/IMC_Auto.IMC_Auto" (struct)))

(fn `UserConstructionScript`
  (bind _box (`self.Box`))
  (bind _returnvalue (`SceneComponent.GetRelativeTransform` _box))
  (`SceneComponent.K2_SetRelativeTransform` _box (`KismetMathLibrary.MakeTransform` (.location _returnvalue) (.rotation _returnvalue) (`KismetMathLibrary.MakeVector` (`self.Return Value Scale X`) (`self.Return Value Scale Y`) (.z (.scale _returnvalue)))) false false)
  (`ShapeComponent.SetLineThickness` (`self.Box`) (`self.Line Thickness`)))