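; BP_Car is a drivable car that applies forward force from move input and sets the mesh's yaw from turn input.
; It records its starting transform on BeginPlay, and ResetAuto restores that transform along with visibility and collision.
; Mesh hits are checked against a Border array: a possessed car calls ResetTimerMessage on BP_AutoTrigger's timer, while an unpossessed one is hidden with collision disabled.
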(event `self.ReceiveBeginPlay`
  (set `self.RefBaseLocation` (`SceneComponent.K2_GetComponentLocation` (`self.StaticMesh`)))
  (set `self.RefBaseRotation` (`SceneComponent.K2_GetComponentRotation` (`self.StaticMesh`)))
  (bind _returnvalue (`GameplayStatics.GetActorOfClass` "/Game/Blueprints/BP_AutoTrigger.BP_AutoTrigger_C"))
  (set `self.RefAutoTrigger` _returnvalue))

(event `/Game/Blueprints/BPI/BPI_Auto.ResetAuto`
  ;[1 1 1] Reset Position Car
  (`self.SetActorHiddenInGame` false)
  (`self.SetActorEnableCollision` true)
  (`SceneComponent.K2_SetRelativeLocationAndRotation` (`self.StaticMesh`) (`self.RefBaseLocation`) (`self.RefBaseRotation`) false false))

(event `EnhancedInput|/Game/ThirdPerson/Input/Actions/IA_AutoMove`
  (params (ActionValue :type "Float (double-precision)") (ElapsedSeconds :type "Float (double-precision)") (TriggeredSeconds :type "Float (double-precision)") (InputAction :type "InputAction Object Reference" :default "/Game/ThirdPerson/Input/Actions/IA_AutoMove.IA_AutoMove"))
  ;[1 1 1] Mouvement
  (:`Triggered`
    (`PrimitiveComponent.AddForce` (`self.StaticMesh`) (* (`SceneComponent.GetForwardVector` (`self.StaticMesh`)) (`self.MoveForce`) ActionValue) "None" false)))

(event `EnhancedInput|/Game/ThirdPerson/Input/Actions/IA_AutoTurn`
  (params (ActionValue :type "Float (double-precision)") (ElapsedSeconds :type "Float (double-precision)") (TriggeredSeconds :type "Float (double-precision)") (InputAction :type "InputAction Object Reference" :default "/Game/ThirdPerson/Input/Actions/IA_AutoTurn.IA_AutoTurn"))
  (bind (_returnvalue_roll _returnvalue_pitch _returnvalue_yaw) (`KismetMathLibrary.BreakRotator` (`SceneComponent.K2_GetComponentRotation` (`self.StaticMesh`))))
  ;[1 1 1] Mouvement
  (:`Triggered`
    (`SceneComponent.K2_SetWorldRotation` (`self.StaticMesh`) (`KismetMathLibrary.MakeRotator` 0.0 0.0 (+ (* ActionValue (`self.TurnSpeed`)) _returnvalue_yaw)) false false)))

(event `self.StaticMesh.OnComponentHit`
  (params (HitComponent :type "PrimitiveComponent Object Reference") (OtherActor :type "Actor Object Reference") (OtherComp :type "PrimitiveComponent Object Reference") (NormalImpulse :type "Vector Structure") (Hit :type "HitResult Structure (by ref)"))
  ;[1 1 1] Détection collision avec un mur
  (for _array_element (`self.Border`)
    (if (== _array_element OtherActor)
      (`|ExecutionSequence`
        (:`then_0`
          (break))
        (:`then_1`
          (set `self.isBorder?` true)
          (`KismetSystemLibrary.PrintString` "Hello")))
      (else
        (set `self.isBorder?` false))))
  (if (`self.isBorder?`)
    (if (`self.isPossed?`)
      (`GameplayStatics.GetActorOfClass` "/Game/Blueprints/BP_AutoTrigger.BP_AutoTrigger_C")
      (message `/Game/Blueprints/BPI/BPI_Auto.ResetTimer` (`/Game/Blueprints/BP_AutoTrigger.RefTimer` (`self.RefAutoTrigger`)))
      (else
        (`self.SetActorHiddenInGame` true)
        (`self.SetActorEnableCollision` false)))))

(event `self.ReceiveTick`
  (params (DeltaSeconds :type "Float (single-precision)")))

(fn `UserConstructionScript`)