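; BP_NPC is an AI pedestrian that wanders between randomly chosen BP_TargetPoints.
; Move rerolls creation points, uses AIMoveTo, then picks again at regular points or destroys the NPC at destruction points.
; A Construction graph spawns new NPCs at BP_SpawnPoint and starts them moving.
; Logic to stop, turn toward the player, greet with sound and resume is disconnected, leaving the Tick proximity check without effect.
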(event `self.ReceiveBeginPlay`
  (bind _returnvalue (`GameplayStatics.GetActorOfClass` "/Game/ThirdPerson/Blueprints/BP_ThirdPersonCharacter.BP_ThirdPersonCharacter_C"))
  (set `self.RefChara` _returnvalue)
  (bind _outactors (`GameplayStatics.GetAllActorsOfClass` "/Game/Blueprints/BP_TargetPoint.BP_TargetPoint_C"))
  (set `self.RefTargetPoint` _outactors)
  (bind _returnvalue_2 (`GameplayStatics.GetActorOfClass` "/Game/Blueprints/BP_SpawnPoint.BP_SpawnPoint_C"))
  (set `self.RefSpawnPoint` _returnvalue_2)
  (`self.Move`)
  (bind _outactors_2 (`GameplayStatics.GetAllActorsOfClass` "/Game/Blueprints/BP_Car.BP_Car_C"))
  (set `self.RefCar` _outactors_2))

(event `/Game/Blueprints/BPI_NPC.StartMoving`
  (params (CurrentEnnemi :type "/Game/Blueprints/BP_NPC Object Reference"))
  (`self.Move` CurrentEnnemi))

(event `Move`
  ;[1 0.3906 0.3906 0.5565] deplacer NPC
  (bind _output_get (set `self.CurrentTarget` (`KismetArrayLibrary.Array_Random` (`self.RefTargetPoint`))))
  (if (`|EnumEquality` (`/Game/Blueprints/BP_TargetPoint.ETarget` _output_get) "NewEnumerator0")
    (`self.Move`)
    (else
      (`|AIMoveTo` self (`self.K2_GetActorLocation` (`self.CurrentTarget`)) null
        (:`OnSuccess`
          (switch `/Game/Blueprints/E_NavTargetPointType` (`/Game/Blueprints/BP_TargetPoint.ETarget` (`self.CurrentTarget`))
            (:`NewEnumerator0`
              (`self.Move`))
            (:`NewEnumerator1`
              (`self.K2_DestroyActor`))
            (:`NewEnumerator2`
              (`self.Move`))))))))

(event `self.ReceiveTick`
  (params (DeltaSeconds :type "Float (single-precision)"))
  ;[1 1 1] Detecter joueur
  (if (< (`KismetMathLibrary.Vector_Distance` (`self.K2_GetActorLocation`) (`SceneComponent.K2_GetComponentLocation` (`Character.CapsuleComponent` (`self.RefChara`)))) 400.0)
    _))

(event `ResetSon`
  ;[1 1 1] Arreter le NPC + le faire se tourner vers le joueur
  (`/Engine/EditorBlueprintResources/StandardMacros.DoOnce` false :!via `Reset`
    (:`Completed`
      (`GameplayStatics.SpawnSoundAtLocation` "/Game/Audio/BONJOUR.BONJOUR" (`self.K2_GetActorLocation` self) (struct) 1.0 1.0 0.0 null null))))

(fn `UserConstructionScript`)