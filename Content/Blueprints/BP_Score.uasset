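; BP_Score is a world actor that displays a score as text on a floating, color-coded mesh.
; CastScore stores the incoming value and updates the text.
; Tick recolors a dynamic M_Score material red for positive scores, green above five and yellow at exactly ten, while ResetColor sets it black.
; A self-restarting Idle timeline animates the actor by adding its offset to the root's height each update.
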(event `AnimIdle`
  (bind (_returnvalue_x _returnvalue_y _returnvalue_z) (`KismetMathLibrary.BreakVector` (`SceneComponent.K2_GetComponentLocation` (`self.DefaultSceneRoot`))))
  (bind (_direction _idle) (`Timeline|Idle` :!via `PlayFromStart`)
    (:`Update`
      (`SceneComponent.K2_SetWorldLocation` (`self.DefaultSceneRoot`) (`KismetMathLibrary.MakeVector` _returnvalue_x _returnvalue_y (+ _returnvalue_z _idle)) false false))
    (:`Finished`
      (`self.AnimIdle`))))

(event `self.ReceiveBeginPlay`
  (bind _returnvalue (`GameplayStatics.GetActorOfClass` "/Game/Blueprints/BP_Target.BP_Target_C"))
  (set `self.RefTarget` _returnvalue)
  (set `self.Value` "0")
  (`self.AnimIdle`)
  (bind _returnvalue_2 (`PrimitiveComponent.CreateDynamicMaterialInstance` (`self.StaticMesh`) 0 "/Game/Materials/M_Score.M_Score" "None"))
  (bind _output_get (set `self.MIScore` _returnvalue_2))
  (`MaterialInstanceDynamic.SetVectorParameterValue` _output_get "Base Color" (`self.ColorBad`)))

(event `/Game/Blueprints/BPI/BPI_Score.CastScore`
  (params (Score :type "Float (double-precision)"))
  (bind _output_get (set `self.ScoreRef` Score))
  (bind _output_get_2 (set `self.Value` (`KismetTextLibrary.Conv_DoubleToText` _output_get "HalfToEven")))
  (`TextRenderComponent.K2_SetText` (`self.Score`) _output_get_2))

(event `self.ReceiveTick`
  (params (DeltaSeconds :type "Float (single-precision)"))
  (if (> (`self.ScoreRef`) 0.0)
    (`MaterialInstanceDynamic.SetVectorParameterValue` (`self.MIScore`) "Base Color" (struct :`R` 1.0 :`A` 1.0))
    (if (> (`self.ScoreRef`) 5.0)
      (`MaterialInstanceDynamic.SetVectorParameterValue` (`self.MIScore`) "Base Color" (struct :`R` 0.015238 :`G` 1.0 :`A` 1.0))
      (if (== (`self.ScoreRef`) 10.0)
        (`MaterialInstanceDynamic.SetVectorParameterValue` (`self.MIScore`) "Base Color" (struct :`R` 0.993859 :`G` 1.0 :`A` 1.0))))))

(event `/Game/Blueprints/BPI/BPI_Score.ResetColor`
  (`MaterialInstanceDynamic.SetVectorParameterValue` (`self.MIScore`) "Base Color" (struct :`A` 1.0)))

(fn `UserConstructionScript`)